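; Component that sends the player's voice and text queries to an AI server over HTTP (VaRest) and shows the results on an NPC or a TV.
; Recordings are uploaded first, then player proximity to the NPC or TV selects text or image generation.
; Generated files are downloaded: runtime-imported WAV plays as the NPC's answer, images become the TV's texture.
; A busy flag rejects overlapping requests, and errors go to the VR pawn's menu or an error widget.
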(event Custom|ImageRequest
  (params (Query%20Content :type String) (Query%20Type :type E_InputType%20Enum :default "NewEnumerator1"))
  ;[0 0 0] Image Generation Request
  (if (Variables|Other|GetEmpty%20request%20queue)
    (Variables|Other|SetEmpty%20request%20queue false)
    (bind _returnvalue (Class|VaRestSubsystem|ConstructVaRestRequestExt (|VaRestSubsystem) "POST" "json"))
    (Class|VaRestRequestJSON|SetRequestObject _returnvalue (|MakeJson (Variables|Server|GetImage%20Model) (Variables|Server|GetSST%20Model) Query%20Content (Utilities|String|EnumtoString Query%20Type)))
    (EventDispatchers|AssignOnRequestComplete _returnvalue (delegate Custom|ImageRequestComplete))
    (EventDispatchers|BindEventtoOnRequestFail _returnvalue (delegate Custom|ImageRequestFail))
    (Class|VaRestRequestJSON|ProcessURL _returnvalue (Utilities|String|ToString(Text) (Utilities|Text|FormatText "http://{0}:{1}/{2}/" (Variables|Server|GetHost%20Address) (Variables|Server|GetHost%20Port) (Variables|Server|GetImage%20URL))))
    (else
      (CallFunction|ShowErrorMessage "Wait for the previous request to finish"))))

(event Custom|TextRequest
  (params (Query%20Content :type String) (Query%20Type :type E_InputType%20Enum :default "NewEnumerator0"))
  ;[0 0 0] Text Generation Request
  (if (Variables|Other|GetEmpty%20request%20queue)
    (Variables|Other|SetEmpty%20request%20queue false)
    (bind _returnvalue (Class|VaRestSubsystem|ConstructVaRestRequestExt (|VaRestSubsystem) "POST" "json"))
    (Class|VaRestRequestJSON|SetRequestObject _returnvalue (|MakeJson (Variables|Server|GetText%20Model) (Variables|Server|GetSST%20Model) (Variables|Server|GetTTS%20Model) (Variables|Server|GetTTS%20Voice) Query%20Content (Utilities|String|EnumtoString Query%20Type)))
    (EventDispatchers|AssignOnRequestComplete _returnvalue (delegate Custom|TextRequestComplete))
    (EventDispatchers|BindEventtoOnRequestFail _returnvalue (delegate Custom|TextRequestFail))
    (Class|VaRestRequestJSON|ProcessURL _returnvalue (Utilities|String|ToString(Text) (Utilities|Text|FormatText "http://{0}:{1}/{2}/" (Variables|Server|GetHost%20Address) (Variables|Server|GetHost%20Port) (Variables|Server|GetText%20URL))))
    (else
      (CallFunction|ShowErrorMessage "Wait for the previous request to finish"))))

(event Custom|Upload%20File%20Complete
  (params (Request :type Va%20Rest%20Request%20JSON%20Object%20Reference))
  (bind _returnvalue (Class|VaRestRequestJSON|GetResponseObject Request))
  (bind _returnvalue_2 (Class|VaRestJsonObject|GetStringField _returnvalue "status"))
  ;[1 0.4471 0.02745] Process Microphone Request
  (if (Utilities|Enum|Equal(Enum) _returnvalue_2 "File uploaded successfully")
    (CallFunction|SendRequest (Class|VaRestJsonObject|GetStringField _returnvalue "filename") "NewEnumerator0")
    (elif (== (Utilities|String|Len _returnvalue_2) 0)
      (CallFunction|ShowErrorMessage "Failed to connect to the server")
      (else
        (CallFunction|ShowErrorMessage (Utilities|Text|ToText(String) _returnvalue_2))))))

(event Custom|Upload%20File%20Fail
  (params (Request :type Va%20Rest%20Request%20JSON%20Object%20Reference))
  ;[1 0.4471 0.02745] Process Microphone Request
  (CallFunction|ShowErrorMessage "An error occurred during the upload of the recording to server"))

(event Custom|TextRequestAudioImport
  (params (Text :type String) (Len :type Float%20%28double-precision%29) (File :type Array%20of%20Bytes))
  ;[0 0 0] Text Generation Request
  (bind _returnvalue (Class|RuntimeAudioImporterLibrary|CreateRuntimeAudioImporter))
  (bind _output_get (Variables|Other|SetAudio%20Importer _returnvalue))
  (EventDispatchers|BindEventtoOnResult _output_get (delegate Custom|TextRequestAudioImportComplete))
  (Class|RuntimeAudioImporterLibrary|ImportAudiofromBuffer (Variables|Other|GetAudio%20Importer) File "Wav"))

(event Custom|TextRequestDownloadAudioComplete
  (params (Request :type Va%20Rest%20Request%20JSON%20Object%20Reference))
  ;[0 0 0] Text Generation Request
  (switch int (Class|VaRestRequestJSON|GetResponseCode Request)
    (:Default
      (CallFunction|ShowErrorMessage "Failed to download audio from server"))
    (:200
      (CallFunction|TextRequestAudioImport (stale Custom|TextRequestDownloadAudio Text) (stale Custom|TextRequestDownloadAudio Len) (Class|VaRestRequestJSON|GetResponseContent Request)))))

(event Custom|TextRequestDownloadAudioFail
  (params (Request :type Va%20Rest%20Request%20JSON%20Object%20Reference))
  ;[0 0 0] Text Generation Request
  (CallFunction|ShowErrorMessage "Unable to download audio file from server"))

(event Custom|TextRequestFail
  (params (Request :type Va%20Rest%20Request%20JSON%20Object%20Reference))
  ;[0 0 0] Text Generation Request
  (CallFunction|ShowErrorMessage "Unable to connect to the server"))

(event Custom|ImageRequestDownloadComplete
  (params (Request :type Va%20Rest%20Request%20JSON%20Object%20Reference))
  ;[0 0 0] Image Generation Request
  (switch int (Class|VaRestRequestJSON|GetResponseCode Request)
    (:Default
      (CallFunction|ShowErrorMessage "Unable to download image file from server"))
    (:200
      (bind _returnvalue (Class|KismetRenderingLibrary|ImportBufferasTexture2D (Class|VaRestRequestJSON|GetResponseContent Request)))
      (Default|ChangeImageTexture (Variables|Output|GetOutput%20Screen) _returnvalue)
      (Variables|Other|SetEmpty%20request%20queue true))))

(event Custom|TextRequestDownloadAudio
  (params (Filename :type String) (Text :type String) (Len :type Float%20%28double-precision%29))
  ;[0 0 0] Text Generation Request
  (bind _returnvalue (Class|VaRestSubsystem|ConstructVaRestRequestExt (|VaRestSubsystem) "GET" "binary"))
  (EventDispatchers|AssignOnRequestComplete _returnvalue (delegate Custom|TextRequestDownloadAudioComplete))
  (EventDispatchers|BindEventtoOnRequestFail _returnvalue (delegate Custom|TextRequestDownloadAudioFail))
  (Class|VaRestRequestJSON|ProcessURL _returnvalue (Utilities|String|ToString(Text) (Utilities|Text|FormatText "http://{0}:{1}/download_file/{2}/" (Variables|Server|GetHost%20Address) (Variables|Server|GetHost%20Port) Filename))))

(event Custom|TextRequestComplete
  (params (Request :type Va%20Rest%20Request%20JSON%20Object%20Reference))
  (bind _returnvalue (Class|VaRestRequestJSON|GetResponseObject Request))
  ;[0 0 0] Text Generation Request
  (bind _keep_executing (CallFunction|ProcessResponseStatus (Class|VaRestJsonObject|GetStringField _returnvalue "status")))
  (if _keep_executing
    (CallFunction|TextRequestDownloadAudio (Class|VaRestJsonObject|GetStringField _returnvalue "filename") (Class|VaRestJsonObject|GetStringField _returnvalue "text") (Class|VaRestJsonObject|GetNumberField _returnvalue "len"))))

(event Custom|ImageRequestFail
  (params (Request :type Va%20Rest%20Request%20JSON%20Object%20Reference))
  ;[0 0 0] Image Generation Request
  (CallFunction|ShowErrorMessage "Unable to connect to the server"))

(event Custom|ImageRequestComplete
  (params (Request :type Va%20Rest%20Request%20JSON%20Object%20Reference))
  (bind _returnvalue (Class|VaRestRequestJSON|GetResponseObject Request))
  ;[0 0 0] Image Generation Request
  (bind _keep_executing (CallFunction|ProcessResponseStatus (Class|VaRestJsonObject|GetStringField _returnvalue "status")))
  (if _keep_executing
    (CallFunction|ImageRequestDownload (Class|VaRestJsonObject|GetStringField _returnvalue "filename"))))

(event Custom|Send%20Request
  (params (Text%20Query :type String) (Query%20Type :type E_InputType%20Enum :default "NewEnumerator0"))
  ;[1 0.4471 0.02745] Send Request (Determin content generation type and send)
  (bind _request_type (CallFunction|DetermineRequestType))
  (switch Utilities|FlowControl|Switch|SwitchonE_RequestType _request_type
    (:NewEnumerator0
      (CallFunction|TextRequest Text%20Query Query%20Type))
    (:NewEnumerator1
      (CallFunction|ImageRequest Text%20Query Query%20Type))
    (:NewEnumerator11
      (CallFunction|ShowErrorMessage "You are too far from NPC or TV to make a request"))))

(event Custom|Process%20Microphone%20Request
  (params (Audio%20Data :type Array%20of%20Bytes))
  ;[1 0.4471 0.02745] Process Microphone Request
  (bind _returnvalue (Class|VaRestSubsystem|ConstructVaRestRequestExt (|VaRestSubsystem) "POST" "binary"))
  (Class|VaRestRequestJSON|SetBinaryRequestContent _returnvalue Audio%20Data)
  (EventDispatchers|AssignOnRequestComplete _returnvalue (delegate Custom|Upload%20File%20Complete))
  (EventDispatchers|BindEventtoOnRequestFail _returnvalue (delegate Custom|Upload%20File%20Fail))
  (Class|VaRestRequestJSON|ProcessURL _returnvalue (Utilities|String|ToString(Text) (Utilities|Text|FormatText "http://{0}:{1}/upload_binary_file/wav/" (Variables|Server|GetHost%20Address) (Variables|Server|GetHost%20Port)))))

(event Custom|ImageRequestDownload
  (params (Filename :type String))
  ;[0 0 0] Image Generation Request
  (bind _returnvalue (Class|VaRestSubsystem|ConstructVaRestRequestExt (|VaRestSubsystem) "GET" "binary"))
  (EventDispatchers|AssignOnRequestComplete _returnvalue (delegate Custom|ImageRequestDownloadComplete))
  (EventDispatchers|BindEventtoOnRequestFail _returnvalue (delegate Custom|ImageRequestDownloadFail))
  (Class|VaRestRequestJSON|ProcessURL _returnvalue (Utilities|String|ToString(Text) (Utilities|Text|FormatText "http://{0}:{1}/download_file/{2}/" (Variables|Server|GetHost%20Address) (Variables|Server|GetHost%20Port) Filename))))

(event Custom|ShowErrorMessage
  (params (Error%20Message :type Text))
  ;[0 1 0.9574] Show Error Message
  (if (Variables|VR|GetVR%20Mode)
    (bind _asbp_vrpawn (Utilities|Casting|CastToBP_VRPawn (Game|Player|GetPlayerPawn 0))
      (:then
        (Variables|/Game/VR/BP_VRPawn.BP_VRPawn_C|SetMenu%20Message%20 _asbp_vrpawn Error%20Message))
      (:CastFailed
        _))
    (else
      (Default|DisplayError (Variables|Output|GetOutput%20Error) Error%20Message)))
  (Variables|Other|SetEmpty%20request%20queue true))

(event Custom|TextRequestAudioImportComplete
  (params (Importer :type Runtime%20Audio%20Importer%20Library%20Object%20Reference) (ImportedSoundWave :type Imported%20Sound%20Wave%20Object%20Reference) (Status :type ERuntimeImportStatus%20Enum :default "SuccessfulImport"))
  ;[0 0 0] Text Generation Request
  (switch Utilities|FlowControl|Switch|SwitchonERuntimeImportStatus Status
    (:SuccessfulImport
      (Default|PlayAnswer (Variables|Output|GetOutput%20NPC) (stale Custom|TextRequestAudioImport Text) (stale Custom|TextRequestAudioImport Len) ImportedSoundWave)
      (Variables|Other|SetEmpty%20request%20queue true))
    (:FailedToReadAudioDataArray
      (CallFunction|ShowErrorMessage (Utilities|Text|ToText(String) (Utilities|String|EnumtoString Status)) :!label _label))
    (:SoundWaveDeclarationError
      (goto _label))
    (:InvalidAudioFormat
      (goto _label))
    (:AudioDoesNotExist
      (goto _label))
    (:LoadFileToArrayError
      (goto _label))))

(event Custom|ImageRequestDownloadFail
  (params (Request :type Va%20Rest%20Request%20JSON%20Object%20Reference))
  ;[0 0 0] Image Generation Request
  (CallFunction|ShowErrorMessage "Server does not respond to image download request"))

(fn SetRequestsValues
  (params (Text%20Model :type String) (Image%20Model :type String) (TTS%20Model :type String) (TTS%20Voice :type String) (SST%20Model :type String) (Host%20Address :type String) (Host%20Port :type String) (Text%20URL :type String) (Image%20URL :type String) (TV%20Reference :type BP%20TV%20Object%20Reference) (NPC%20Reference :type BP%20NPC%20Object%20Reference) (Error%20Widget%20Reference :type WBP%20Error%20Object%20Reference) (Player%20Location :type Vector) (VR%20Mode :type Boolean))
  (Variables|Server|SetText%20Model Text%20Model)
  (Variables|Server|SetImage%20Model Image%20Model)
  (Variables|Server|SetTTS%20Model TTS%20Model)
  (Variables|Server|SetTTS%20Voice TTS%20Voice)
  (Variables|Server|SetSST%20Model SST%20Model)
  (Variables|Server|SetHost%20Address Host%20Address)
  (Variables|Server|SetHost%20Port Host%20Port)
  (Variables|Server|SetText%20URL Text%20URL)
  (Variables|Server|SetImage%20URL Image%20URL)
  (Variables|Output|SetOutput%20Screen TV%20Reference)
  (Variables|Output|SetOutput%20NPC NPC%20Reference)
  (Variables|Output|SetOutput%20Error Error%20Widget%20Reference)
  (Variables|Other|SetPlayer%20Location Player%20Location)
  (Variables|VR|SetVR%20Mode VR%20Mode))

(fn ProcessResponseStatus
  (params (Status :type String))
  (bind _returnvalue (Utilities|Enum|Equal(Enum) Status "Text generated successfully"))
  (bind _returnvalue_2 (Utilities|Enum|Equal(Enum) Status "Image generated successfully"))
  (bind _returnvalue_3 (or _returnvalue _returnvalue_2))
  (if _returnvalue_3
    _
    (elif (== (Utilities|String|Len Status) 0)
      (CallFunction|ShowErrorMessage "Failed to connect to the server")
      (else
        (CallFunction|ShowErrorMessage (Utilities|Text|ToText(String) Status)))))
  (return _returnvalue_3))

(fn DetermineRequestType
  (bind _player_location (Variables|Other|GetPlayer%20Location))
  (LocalVariables|SetDistance%20To%20TV (Math|Vector|Distance(Vector) _player_location (Transformation|GetWorldLocation (Variables|/Game/Blueprints/Interaction/BP_TV.BP_TV_C|GetScreen (Variables|Output|GetOutput%20Screen)))))
  (LocalVariables|SetDistance%20To%20NPC (Math|Vector|Distance(Vector) _player_location (Transformation|GetWorldLocation (Variables|/Game/Blueprints/BP_NPC.BP_NPC_C|GetBody (Variables|Output|GetOutput%20NPC)))))
  (if (and (>= (LocalVariables|GetDistance%20To%20TV) (LocalVariables|GetMax%20acceptable%20distance)) (>= (LocalVariables|GetDistance%20To%20NPC) (LocalVariables|GetMax%20acceptable%20distance)))
    (return "NewEnumerator11")
    (elif (>= (LocalVariables|GetDistance%20To%20TV) (LocalVariables|GetDistance%20To%20NPC))
      (return "NewEnumerator0")
      (else
        (return "NewEnumerator1")))))