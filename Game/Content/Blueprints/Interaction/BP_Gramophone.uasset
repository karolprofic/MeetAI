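; BP_Gramophone is an interactable gramophone that toggles the music playing on the player's BP_Character and animates its moving parts.
; TurnOnOffMusic swings the reader arm through a timeline on first activation, starts or pauses the music, and drives a looping RotateVinyl timer that spins the record.
; A box collision swaps the character's general interaction widget for the gramophone controls widget while the player overlaps it.
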(event OnComponentBeginOverlap(BoxCollision)
  (params (OverlappedComponent :type Primitive%20Component%20Object%20Reference) (OtherActor :type Actor%20Object%20Reference) (OtherComp :type Primitive%20Component%20Object%20Reference) (OtherBodyIndex :type Integer) (bFromSweep :type Boolean) (SweepResult :type Hit%20Result%20Structure%20%28by%20ref%29))
  ;[1 1 1] Show / Hide controls
  (bind _asbp_character (Utilities|Casting|CastToBP_Character OtherActor))
  (Widget|SetVisibility (Variables|/Game/Blueprints/BP_Character.BP_Character_C|GetGramophoneWidget _asbp_character) "Visible")
  (Widget|SetVisibility (Variables|/Game/Blueprints/BP_Character.BP_Character_C|GetInteractionWidget _asbp_character) "Hidden"))

(event OnComponentEndOverlap(BoxCollision)
  (params (OverlappedComponent :type Primitive%20Component%20Object%20Reference) (OtherActor :type Actor%20Object%20Reference) (OtherComp :type Primitive%20Component%20Object%20Reference) (OtherBodyIndex :type Integer))
  ;[1 1 1] Show / Hide controls
  (bind _asbp_character (Utilities|Casting|CastToBP_Character OtherActor))
  (Widget|SetVisibility (Variables|/Game/Blueprints/BP_Character.BP_Character_C|GetGramophoneWidget _asbp_character) "Hidden")
  (Widget|SetVisibility (Variables|/Game/Blueprints/BP_Character.BP_Character_C|GetInteractionWidget _asbp_character) "Visible")
  (Variables|/Game/Widgets/WBP_Interaction.WBP_Interaction_C|SetInteraction%20Text (Variables|/Game/Blueprints/BP_Character.BP_Character_C|GetInteractionWidget _asbp_character) ""))

(event Custom|RotateVinyl
  ;[1 1 1] Rotate vinyl
  (Transformation|AddRelativeRotation (Variables|Default|GetRecordRotationPoint) "0,5.000000, 0" false false))

(event Custom|TurnOnOffMusic
  ;[1 1 1] Turn on / off music
  (if (Variables|Default|GetIsMusicPlaying)
    (Class|KismetSystemLibrary|PauseTimer 0 "RotateVinyl")
    (Variables|Default|SetIsMusicPlaying false)
    (bind _asbp_character (Utilities|Casting|CastToBP_Character (Game|Player|GetPlayerPawn 0)))
    (Class|AudioComponent|SetPaused (Variables|/Game/Blueprints/BP_Character.BP_Character_C|GetMusic _asbp_character) true)
    (else
      (if (Variables|Default|GetFirstActivation)
        (bind _readerrotation (Timeline|Timeline Play)
          (:Update
            (Transformation|SetRelativeRotation (Variables|Default|GetReaderRotationPoint) (Math|Rotator|MakeRotator 9e+01 0.0 (Math|Float|Lerp 0.0 41.0 _readerrotation)) false false)
            (Variables|Default|SetFirstActivation false))))
      (Utilities|Time|SetTimerbyFunctionName 0 "RotateVinyl" 0.03 true)
      (Variables|Default|SetIsMusicPlaying true)
      (bind _asbp_character_2 (Utilities|Casting|CastToBP_Character (Game|Player|GetPlayerPawn 0)))
      (Audio|Components|Audio|Play (Variables|/Game/Blueprints/BP_Character.BP_Character_C|GetMusic _asbp_character_2) 0.0)
      (Class|AudioComponent|SetPaused (Variables|/Game/Blueprints/BP_Character.BP_Character_C|GetMusic _asbp_character_2) false))))

(fn ConstructionScript)