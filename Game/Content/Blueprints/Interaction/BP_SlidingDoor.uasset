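; Interactable sliding door that shows the player an open/close prompt while their BP_Character overlaps its box collision.
; OpenOrCloseDoor, with no caller in this graph, updates the prompt, plays a sound and runs a timeline forward or in reverse based on IsOpen.
; The timeline slides the door along X and tilts the handle pivot on separate tracks.
; On finish it toggles IsOpen and IsAudioPlaying, the flag gating the sound.
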(event OnComponentBeginOverlap(BoxCollision)
  (params (OverlappedComponent :type Primitive%20Component%20Object%20Reference) (OtherActor :type Actor%20Object%20Reference) (OtherComp :type Primitive%20Component%20Object%20Reference) (OtherBodyIndex :type Integer) (bFromSweep :type Boolean) (SweepResult :type Hit%20Result%20Structure%20%28by%20ref%29))
  ;[1 1 1] Show widget
  (bind _asbp_character (Utilities|Casting|CastToBP_Character OtherActor))
  (Variables|/Game/Widgets/WBP_Interaction.WBP_Interaction_C|SetInteraction%20Text (Variables|/Game/Blueprints/BP_Character.BP_Character_C|GetInteractionWidget _asbp_character) (Variables|Default|GetPromptText))
  (Widget|SetVisibility (Variables|/Game/Blueprints/BP_Character.BP_Character_C|GetInteractionWidget _asbp_character) "Visible"))

(event OnComponentEndOverlap(BoxCollision)
  (params (OverlappedComponent :type Primitive%20Component%20Object%20Reference) (OtherActor :type Actor%20Object%20Reference) (OtherComp :type Primitive%20Component%20Object%20Reference) (OtherBodyIndex :type Integer))
  ;[1 1 1] Hide widget
  (bind _asbp_character (Utilities|Casting|CastToBP_Character OtherActor))
  (Widget|SetVisibility (Variables|/Game/Blueprints/BP_Character.BP_Character_C|GetInteractionWidget _asbp_character) "Hidden"))

(event Custom|PlaySound
  ;[1 1 1] Play sound
  (if (not (Variables|Default|GetIsAudioPlaying))
    (Audio|PlaySoundatLocation "/Game/Audio/SC_DoorClose.SC_DoorClose" "0, 0, 0" "0, 0, 0" 1.0 1.0 0.0 0 0 0 0)
    (Variables|Default|SetIsAudioPlaying (not (Variables|Default|GetIsAudioPlaying)))))

(event Custom|OpenOrCloseDoor
  ;[1 1 1] Open or close door
  (CallFunction|ChangeDisplayedText)
  (CallFunction|PlaySound)
  (if (Variables|Default|GetIsOpen)
    (bind (_direction _doorfloat _handlerfloat) (Timeline|DoorTimeline Play)
      (:Update
        (Transformation|SetRelativeLocation (Variables|Default|GetDoor) (Math|Vector|MakeVector (Math|Float|Lerp 0.0 -77.0 _doorfloat) 0.0 0.0) false false)
        (Transformation|SetRelativeRotation (Variables|Default|GetRotationPoint) (Math|Rotator|MakeRotator 9e+01 (Math|Float|Lerp 0.0 -15.0 _handlerfloat) 0.0) false false))
      (:Finished
        (Variables|Default|SetIsOpen (not (Variables|Default|GetIsOpen)))
        (Variables|Default|SetIsAudioPlaying (not (Variables|Default|GetIsAudioPlaying)))))
    (else
      (Timeline|DoorTimeline Reverse))))

(event Custom|ChangeDisplayedText
  ;[1 1 1] Change displayed text
  (bind _asbp_character (Utilities|Casting|CastToBP_Character (Game|Player|GetPlayerPawn 0)))
  (if (not (Variables|Default|GetIsOpen))
    (bind _output_get (Variables|/Game/Widgets/WBP_Interaction.WBP_Interaction_C|SetInteraction%20Text (Variables|/Game/Blueprints/BP_Character.BP_Character_C|GetInteractionWidget _asbp_character) "Press Interaction button to close the door"))
    (Variables|Default|SetPromptText _output_get)
    (else
      (bind _output_get_2 (Variables|/Game/Widgets/WBP_Interaction.WBP_Interaction_C|SetInteraction%20Text (Variables|/Game/Blueprints/BP_Character.BP_Character_C|GetInteractionWidget _asbp_character) "Press Interaction button to open the door"))
      (Variables|Default|SetPromptText _output_get_2))))

(fn ConstructionScript)