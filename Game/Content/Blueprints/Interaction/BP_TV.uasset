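; BP_TV is an interactable TV that displays an image supplied as a URL or texture.
; ChangeImagePath downloads the image and ChangeImageTexture takes a texture directly, each applying it through a new M_Download dynamic material instance on the Screen.
; Its BoxCollider shows BP_Character's interaction prompt for opening a text panel or describing an image by voice, and hides it on exit.
; The key input itself is not handled here.
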(event OnComponentBeginOverlap(BoxCollider)
  (params (OverlappedComponent :type Primitive%20Component%20Object%20Reference) (OtherActor :type Actor%20Object%20Reference) (OtherComp :type Primitive%20Component%20Object%20Reference) (OtherBodyIndex :type Integer) (bFromSweep :type Boolean) (SweepResult :type Hit%20Result%20Structure%20%28by%20ref%29))
  (bind _asbp_character (Utilities|Casting|CastToBP_Character OtherActor))
  (Variables|/Game/Widgets/WBP_Interaction.WBP_Interaction_C|SetInteraction%20Text (Variables|/Game/Blueprints/BP_Character.BP_Character_C|GetInteractionWidget _asbp_character) "Press Q to open text panel or hold M to describe image by voice")
  (Widget|SetVisibility (Variables|/Game/Blueprints/BP_Character.BP_Character_C|GetInteractionWidget _asbp_character) "Visible"))

(event OnComponentEndOverlap(BoxCollider)
  (params (OverlappedComponent :type Primitive%20Component%20Object%20Reference) (OtherActor :type Actor%20Object%20Reference) (OtherComp :type Primitive%20Component%20Object%20Reference) (OtherBodyIndex :type Integer))
  (bind _asbp_character (Utilities|Casting|CastToBP_Character OtherActor))
  (Widget|SetVisibility (Variables|/Game/Blueprints/BP_Character.BP_Character_C|GetInteractionWidget _asbp_character) "Hidden"))

(event Custom|Change%20Image%20Texture
  (params (Texture :type Texture%20Object%20Reference))
  (bind _returnvalue (Rendering|Material|CreateDynamicMaterialInstance (Variables|Default|GetScreen) 0 "/Game/Materials/M_Download.M_Download" "None" :!class /Script/Engine.PrimitiveComponent))
  (Rendering|Material|SetTextureParameterValue _returnvalue "Texture" Texture))

(event Custom|Change%20Image%20Path
  (params (URL :type String))
  (bind _texture (|DownloadImage URL)
    (:OnSuccess
      (bind _returnvalue (Rendering|Material|CreateDynamicMaterialInstance (Variables|Default|GetScreen) 0 "/Game/Materials/M_Download.M_Download" "None" :!class /Script/Engine.PrimitiveComponent))
      (Rendering|Material|SetTextureParameterValue _returnvalue "Texture" _texture))))

(fn ConstructionScript)