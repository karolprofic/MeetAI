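; BP_Door is an interactive hinged door that shows an open or close prompt to desktop and VR players.
; Box overlaps set or clear the pawn's InteractionWidget text.
; OpenOrCloseDoor updates that prompt, plays a guarded sound, and runs one timeline forward or in reverse to rotate door and handle.
; The timeline's finish toggles the open and audio-playing flags.
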(event OnComponentBeginOverlap(BoxCollision)
  (params (OverlappedComponent :type Primitive%20Component%20Object%20Reference) (OtherActor :type Actor%20Object%20Reference) (OtherComp :type Primitive%20Component%20Object%20Reference) (OtherBodyIndex :type Integer) (bFromSweep :type Boolean) (SweepResult :type Hit%20Result%20Structure%20%28by%20ref%29))
  ;[1 1 1] Adding widget
  (bind _asbp_player_character (Utilities|Casting|CastToBP_PlayerCharacter OtherActor)
    (:then
      (Variables|/Game/Widgets/WBP_Interaction.WBP_Interaction_C|SetTextToDisplay (Variables|/Game/Blueprints/BP_PlayerCharacter.BP_PlayerCharacter_C|GetInteraction%20Widget _asbp_player_character) (Variables|Default|GetPromptText)))
    (:CastFailed
      ;;[0 0 0] VR
      (bind _asbp_vrpawn (Utilities|Casting|CastToBP_VRPawn OtherActor))
      (Variables|/Game/Widgets/WBP_Interaction.WBP_Interaction_C|SetTextToDisplay (Variables|/Game/VR/Blueprints/BP_VRPawn.BP_VRPawn_C|GetInteraction%20Widget _asbp_vrpawn) (Variables|Default|GetPromptText)))))

(event OnComponentEndOverlap(BoxCollision)
  (params (OverlappedComponent :type Primitive%20Component%20Object%20Reference) (OtherActor :type Actor%20Object%20Reference) (OtherComp :type Primitive%20Component%20Object%20Reference) (OtherBodyIndex :type Integer))
  ;[1 1 1] Removing widget
  (bind _asbp_player_character (Utilities|Casting|CastToBP_PlayerCharacter OtherActor)
    (:then
      (Variables|/Game/Widgets/WBP_Interaction.WBP_Interaction_C|SetTextToDisplay (Variables|/Game/Blueprints/BP_PlayerCharacter.BP_PlayerCharacter_C|GetInteraction%20Widget _asbp_player_character) ""))
    (:CastFailed
      ;;[0 0 0] VR
      (bind _asbp_vrpawn (Utilities|Casting|CastToBP_VRPawn OtherActor))
      (Variables|/Game/Widgets/WBP_Interaction.WBP_Interaction_C|SetTextToDisplay (Variables|/Game/VR/Blueprints/BP_VRPawn.BP_VRPawn_C|GetInteraction%20Widget _asbp_vrpawn) ""))))

(event Custom|PlaySound
  ;[1 1 1] Play sound
  (if (not (Variables|Default|GetIsAudioPlaying))
    (Audio|PlaySoundatLocation "/Game/Audio/SC_DoorClose.SC_DoorClose" "0, 0, 0" "0, 0, 0" 1.0 1.0 0.0 0 0 0 0)
    (Variables|Default|SetIsAudioPlaying (not (Variables|Default|GetIsAudioPlaying)))))

(event Custom|ChangeDisplayedText
  (bind _returnvalue (Game|Player|GetPlayerPawn 0))
  ;[1 1 1] Change displayed text
  (bind _asbp_player_character (Utilities|Casting|CastToBP_PlayerCharacter _returnvalue)
    (:then
      (if (not (Variables|Default|GetIsOpen))
        (bind _output_get (Variables|/Game/Widgets/WBP_Interaction.WBP_Interaction_C|SetTextToDisplay (Variables|/Game/Blueprints/BP_PlayerCharacter.BP_PlayerCharacter_C|GetInteraction%20Widget _asbp_player_character) "Press F to close the door"))
        (Variables|Default|SetPromptText _output_get)
        (else
          (bind _output_get_2 (Variables|/Game/Widgets/WBP_Interaction.WBP_Interaction_C|SetTextToDisplay (Variables|/Game/Blueprints/BP_PlayerCharacter.BP_PlayerCharacter_C|GetInteraction%20Widget _asbp_player_character) "Press F to open the door"))
          (Variables|Default|SetPromptText _output_get_2))))
    (:CastFailed
      ;;[0 0 0] VR
      (bind _asbp_vrpawn (Utilities|Casting|CastToBP_VRPawn _returnvalue))
      (if (not (Variables|Default|GetIsOpen))
        (bind _output_get_3 (Variables|/Game/Widgets/WBP_Interaction.WBP_Interaction_C|SetTextToDisplay (Variables|/Game/VR/Blueprints/BP_VRPawn.BP_VRPawn_C|GetInteraction%20Widget _asbp_vrpawn) "Press F to close the door"))
        (Variables|Default|SetPromptText _output_get_3)
        (else
          (bind _output_get_4 (Variables|/Game/Widgets/WBP_Interaction.WBP_Interaction_C|SetTextToDisplay (Variables|/Game/VR/Blueprints/BP_VRPawn.BP_VRPawn_C|GetInteraction%20Widget _asbp_vrpawn) "Press F to open the door"))
          (Variables|Default|SetPromptText _output_get_4))))))

(event Custom|OpenOrCloseDoor
  ;[1 1 1] Open or close door
  (CallFunction|ChangeDisplayedText)
  (CallFunction|PlaySound)
  (if (Variables|Default|GetIsOpen)
    (bind (_direction _doorfloat _handlerfloat) (Timeline|Timeline_0 Play)
      (:Update
        (Transformation|SetRelativeRotation (Variables|Default|GetDoorRotationPoint) (Math|Rotator|MakeRotator 0.0 0.0 (Math|Float|Lerp 1.1e+02 0.0 _doorfloat)) false false)
        (Transformation|SetRelativeRotation (Variables|Default|GetHandlerRotationPoint) (Math|Rotator|MakeRotator 0.0 (Math|Float|Lerp 0.0 -15.0 _handlerfloat) 0.0) false false))
      (:Finished
        (Variables|Default|SetIsOpen (not (Variables|Default|GetIsOpen)))
        (Variables|Default|SetIsAudioPlaying (not (Variables|Default|GetIsAudioPlaying)))))
    (else
      (Timeline|Timeline_0 Reverse))))

(fn ConstructionScript)