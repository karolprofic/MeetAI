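; BP_Gramophone is an interactive gramophone that turns music on and off for either the desktop character or VR pawn.
; TurnOnOffMusic toggles the Music component on the player pawn, starting or pausing a looping timer that spins the record.
; On first activation, a Timeline swings the reader arm onto the record while starting playback.
; Box collision overlaps swap the pawn's gramophone controls widget with its interaction widget.
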(event OnComponentBeginOverlap(BoxCollision)
  (params (OverlappedComponent :type Primitive%20Component%20Object%20Reference) (OtherActor :type Actor%20Object%20Reference) (OtherComp :type Primitive%20Component%20Object%20Reference) (OtherBodyIndex :type Integer) (bFromSweep :type Boolean) (SweepResult :type Hit%20Result%20Structure%20%28by%20ref%29))
  ;[1 1 1] Show / Hide controls
  (bind _asbp_player_character (Utilities|Casting|CastToBP_PlayerCharacter OtherActor)
    (:then
      (Widget|SetVisibility (Variables|/Game/Blueprints/BP_PlayerCharacter.BP_PlayerCharacter_C|GetGramophone%20Widget _asbp_player_character) "Visible")
      (Widget|SetVisibility (Variables|/Game/Blueprints/BP_PlayerCharacter.BP_PlayerCharacter_C|GetInteraction%20Widget _asbp_player_character) "Hidden"))
    (:CastFailed
      ;;[0 0 0] VR
      (bind _asbp_vrpawn (Utilities|Casting|CastToBP_VRPawn OtherActor))
      (Widget|SetVisibility (Variables|/Game/VR/Blueprints/BP_VRPawn.BP_VRPawn_C|GetGramophone%20Widget _asbp_vrpawn) "Visible")
      (Widget|SetVisibility (Variables|/Game/VR/Blueprints/BP_VRPawn.BP_VRPawn_C|GetInteraction%20Widget _asbp_vrpawn) "Hidden"))))

(event OnComponentEndOverlap(BoxCollision)
  (params (OverlappedComponent :type Primitive%20Component%20Object%20Reference) (OtherActor :type Actor%20Object%20Reference) (OtherComp :type Primitive%20Component%20Object%20Reference) (OtherBodyIndex :type Integer))
  ;[1 1 1] Show / Hide controls
  (bind _asbp_player_character (Utilities|Casting|CastToBP_PlayerCharacter OtherActor)
    (:then
      (Widget|SetVisibility (Variables|/Game/Blueprints/BP_PlayerCharacter.BP_PlayerCharacter_C|GetGramophone%20Widget _asbp_player_character) "Hidden")
      (Widget|SetVisibility (Variables|/Game/Blueprints/BP_PlayerCharacter.BP_PlayerCharacter_C|GetInteraction%20Widget _asbp_player_character) "Visible"))
    (:CastFailed
      ;;[0 0 0] VR
      (bind _asbp_vrpawn (Utilities|Casting|CastToBP_VRPawn OtherActor))
      (Widget|SetVisibility (Variables|/Game/VR/Blueprints/BP_VRPawn.BP_VRPawn_C|GetGramophone%20Widget _asbp_vrpawn) "Hidden")
      (Widget|SetVisibility (Variables|/Game/VR/Blueprints/BP_VRPawn.BP_VRPawn_C|GetInteraction%20Widget _asbp_vrpawn) "Visible"))))

(event Custom|RotateVinyl
  ;[1 1 1] Rotate vinyl
  (Transformation|AddRelativeRotation (Variables|Default|GetRecordRotationPoint) "0,5.000000, 0" false false))

(event Custom|TurnOnOffMusic
  (bind _returnvalue (Game|Player|GetPlayerPawn 0))
  (bind _returnvalue_2 (Game|Player|GetPlayerPawn 0))
  ;[1 1 1] Turn on / off music
  (if (Variables|Default|GetIsMusicPlaying)
    (Class|KismetSystemLibrary|PauseTimer 0 "RotateVinyl")
    (Variables|Default|SetIsMusicPlaying false)
    (bind _asbp_player_character (Utilities|Casting|CastToBP_PlayerCharacter _returnvalue_2)
      (:then
        (Class|AudioComponent|SetPaused (Variables|/Game/Blueprints/BP_PlayerCharacter.BP_PlayerCharacter_C|GetMusic _asbp_player_character) true))
      (:CastFailed
        ;;[0 0 0] VR
        (bind _asbp_vrpawn (Utilities|Casting|CastToBP_VRPawn _returnvalue_2))
        (Class|AudioComponent|SetPaused (Variables|/Game/VR/Blueprints/BP_VRPawn.BP_VRPawn_C|GetMusic _asbp_vrpawn) true)))
    (else
      (if (Variables|Default|GetFirstActivation)
        (bind _readerrotation (Timeline|Timeline Play)
          (:Update
            (Transformation|SetRelativeRotation (Variables|Default|GetReaderRotationPoint) (Math|Rotator|MakeRotator 9e+01 0.0 (Math|Float|Lerp 0.0 41.0 _readerrotation)) false false)
            (Variables|Default|SetFirstActivation false))))
      (Utilities|Time|SetTimerbyFunctionName 0 "RotateVinyl" 0.03 true)
      (Variables|Default|SetIsMusicPlaying true)
      (bind _asbp_player_character_2 (Utilities|Casting|CastToBP_PlayerCharacter _returnvalue)
        (:then
          (Audio|Components|Audio|Play (Variables|/Game/Blueprints/BP_PlayerCharacter.BP_PlayerCharacter_C|GetMusic _asbp_player_character_2) 0.0)
          (Class|AudioComponent|SetPaused (Variables|/Game/Blueprints/BP_PlayerCharacter.BP_PlayerCharacter_C|GetMusic _asbp_player_character_2) false))
        (:CastFailed
          ;;[0 0 0] VR
          (bind _asbp_vrpawn_2 (Utilities|Casting|CastToBP_VRPawn _returnvalue))
          (Audio|Components|Audio|Play (Variables|/Game/VR/Blueprints/BP_VRPawn.BP_VRPawn_C|GetMusic _asbp_vrpawn_2) 0.0)
          (Class|AudioComponent|SetPaused (Variables|/Game/VR/Blueprints/BP_VRPawn.BP_VRPawn_C|GetMusic _asbp_vrpawn_2) false))))))

(fn ConstructionScript)