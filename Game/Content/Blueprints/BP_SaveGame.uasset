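; BP_SaveGame is a save game data container for the player's graphics, AI and audio settings.
; Each category has a Save function that copies its inputs into member variables and a Load function that returns them.
; Graphics options keep paired setting and Value fields, plus VSync and VR mode values, while AI settings hold an address, port, and text, image and conversational model choices.
; The file itself performs no disk I/O or applying of settings.
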(fn LoadGraphicsSettings
  (return (Variables|Default|GetResolution) (Variables|Default|GetWindow%20Mode) (Variables|Default|GetMax%20FPS) (Variables|Default|GetViewDistance) (Variables|Default|GetTextures) (Variables|Default|GetPost-Processing) (Variables|Default|GetShadows) (Variables|Default|GetEffects) (Variables|Default|GetFoliage) (Variables|Default|GetResolution%20Value) (Variables|Default|GetWindow%20Mode%20Value) (Variables|Default|GetMax%20FPS%20Value) (Variables|Default|GetViewDistance%20Value) (Variables|Default|GetTextures%20Value) (Variables|Default|GetPost-Processing%20Value) (Variables|Default|GetShadows%20Value) (Variables|Default|GetEffects%20Value) (Variables|Default|GetFoliage%20Value) (Variables|Default|GetV-Sync%20Value) (Variables|Default|GetVR%20Mode%20Value)))

(fn SaveGraphicsSettings
  (params (Resolution :type String) (Window%20Mode :type String) (Max%20FPS :type String) (ViewDistance :type String) (Textures :type String) (Foliage :type String) (Post-Processing :type String) (Shadows :type String) (Effects :type String) (Resolution%20Value :type Integer) (Window%20Mode%20Value :type Integer) (Max%20FPS%20Value :type Integer) (ViewDistance%20Value :type Integer) (Foliage%20Value :type Integer) (Textures%20Value :type Integer) (Post-Processing%20Value :type Integer) (Shadows%20Value :type Integer) (Effects%20Value :type Integer) (V-Sync%20Value :type Boolean) (VR%20Mode%20Value :type Boolean))
  (Variables|Default|SetResolution Resolution)
  (Variables|Default|SetWindow%20Mode Window%20Mode)
  (Variables|Default|SetMax%20FPS Max%20FPS)
  (Variables|Default|SetViewDistance ViewDistance)
  (Variables|Default|SetTextures Textures)
  (Variables|Default|SetFoliage Foliage)
  (Variables|Default|SetPost-Processing Post-Processing)
  (Variables|Default|SetShadows Shadows)
  (Variables|Default|SetEffects Effects)
  (Variables|Default|SetResolution%20Value Resolution%20Value)
  (Variables|Default|SetWindow%20Mode%20Value Window%20Mode%20Value)
  (Variables|Default|SetMax%20FPS%20Value Max%20FPS%20Value)
  (Variables|Default|SetViewDistance%20Value ViewDistance%20Value)
  (Variables|Default|SetTextures%20Value Textures%20Value)
  (Variables|Default|SetPost-Processing%20Value Post-Processing%20Value)
  (Variables|Default|SetShadows%20Value Shadows%20Value)
  (Variables|Default|SetFoliage%20Value Foliage%20Value)
  (Variables|Default|SetEffects%20Value Effects%20Value)
  (Variables|Default|SetV-Sync%20Value V-Sync%20Value)
  (Variables|Default|SetVR%20Mode%20Value VR%20Mode%20Value))

(fn LoadAISettings
  (return (Variables|Default|GetAI_Address) (Variables|Default|GetAI_Port) (Variables|Default|GetAI_TextModel) (Variables|Default|GetAI_ImageModel) (Variables|Default|GetAI_ConversationalModel)))

(fn SaveAISettings
  (params (AI_Address :type Text) (AI_Port :type Text) (AI_TextModel :type Text) (AI_ImageModel :type Text) (AI_ConversationalModel :type Text))
  (Variables|Default|SetAI_Address AI_Address)
  (Variables|Default|SetAI_Port AI_Port)
  (Variables|Default|SetAI_TextModel AI_TextModel)
  (Variables|Default|SetAI_ImageModel AI_ImageModel)
  (Variables|Default|SetAI_ConversationalModel AI_ConversationalModel))

(fn LoadAudioSettings
  (return (Variables|Default|GetAudio_Speech%20) (Variables|Default|GetAudio_Music) (Variables|Default|GetAudio_Effects)))

(fn SaveAudioSettings
  (params (Audio_Speech%20 :type Float%20%28double-precision%29) (Audio_Music :type Float%20%28double-precision%29) (Audio_Effects :type Float%20%28double-precision%29))
  (Variables|Default|SetAudio_Speech%20 Audio_Speech%20)
  (Variables|Default|SetAudio_Music Audio_Music)
  (Variables|Default|SetAudio_Effects Audio_Effects))